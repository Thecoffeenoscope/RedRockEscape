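; Editor ruler actor that labels the segment lengths of a spline with floating text.
; The construction script, gated by a toggle, loops over spline points and measures distance from each previous point.
; It adds a text render component at each segment midpoint, raised by a vertical offset and sized in proportion to segment length.
; A unit enum switches the readout between Unreal units and meters.
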(event EventBeginPlay)

(event Collision|EventActorBeginOverlap
  (params (OtherActor :type Actor%20Object%20Reference)))

(event EventTick
  (params (DeltaSeconds :type Float%20%28single-precision%29)))

(fn ConstructionScript
  (bind _spline (Variables|Default|GetSpline))
  (if (Variables|Default|GetToggleMesurements)
    (Variables|Default|SetNumOfSplinePoints (Spline|GetNumberOfSplinePoints (Variables|Default|GetSpline)))
    (for _index (range 0 (Variables|Default|GetNumOfSplinePoints))
      (Variables|Default|SetCurrentPointIndex _index)
      (if (!= (Variables|Default|GetCurrentPointIndex) (Variables|Default|GetNumOfSplinePoints))
        ;[0.15 0.15 0.15 0.5] Get Length of spline
        (Variables|Default|SetSegmentLengthUU (- (Spline|GetDistanceAlongSplineatSplinePoint _spline (Variables|Default|GetCurrentPointIndex)) (Spline|GetDistanceAlongSplineatSplinePoint _spline (- (Variables|Default|GetCurrentPointIndex) 1))))
        (bind _returnvalue (AddComponent|AddTextRenderComponent false (Math|Transform|MakeTransform (Math|Vector|MakeVector (.x (Spline|GetLocationatDistanceAlongSpline (Variables|Default|GetSpline) (+ (/ (- (Spline|GetDistanceAlongSplineatSplinePoint _spline (Variables|Default|GetCurrentPointIndex)) (Spline|GetDistanceAlongSplineatSplinePoint _spline (- (Variables|Default|GetCurrentPointIndex) 1))) 2.0) (Spline|GetDistanceAlongSplineatSplinePoint _spline (- (Variables|Default|GetCurrentPointIndex) 1))) "Local")) (.y (Spline|GetLocationatDistanceAlongSpline (Variables|Default|GetSpline) (+ (/ (- (Spline|GetDistanceAlongSplineatSplinePoint _spline (Variables|Default|GetCurrentPointIndex)) (Spline|GetDistanceAlongSplineatSplinePoint _spline (- (Variables|Default|GetCurrentPointIndex) 1))) 2.0) (Spline|GetDistanceAlongSplineatSplinePoint _spline (- (Variables|Default|GetCurrentPointIndex) 1))) "Local")) (+ (.z (Spline|GetLocationatDistanceAlongSpline (Variables|Default|GetSpline) (+ (/ (- (Spline|GetDistanceAlongSplineatSplinePoint _spline (Variables|Default|GetCurrentPointIndex)) (Spline|GetDistanceAlongSplineatSplinePoint _spline (- (Variables|Default|GetCurrentPointIndex) 1))) 2.0) (Spline|GetDistanceAlongSplineatSplinePoint _spline (- (Variables|Default|GetCurrentPointIndex) 1))) "Local")) (Variables|Default|GetTextVertialOffset))) "0, 0, 0" "1.000000,1.000000,1.000000")))
        (bind _output_get (Variables|Default|SetTextReff _returnvalue))
        (Transformation|SetAbsolute _output_get false false false)
        (Rendering|Components|TextRender|SetWorldSize (Variables|Default|GetTextReff) (* (Variables|Default|GetSegmentLengthUU) (Variables|Default|GetDefualtSizeMultipilier)))
        ;[0.15 0.15 0.15 0.5] Check which mesurement system to use.
        (if (Utilities|Enum|Equal(Enum) (Variables|Default|GetUnitTypes) "NewEnumerator0")
          (Rendering|Components|TextRender|SetText (Variables|Default|GetTextReff) (|GenerictoText (Utilities|String|Append (Utilities|String|ToString(Text) (Utilities|Text|ToText(Float) (Variables|Default|GetSegmentLengthUU) "HalfToEven" false true 1 324 2 2)) "uu")))
          (elif (Utilities|Enum|Equal(Enum) (Variables|Default|GetUnitTypes) "NewEnumerator1")
            (Rendering|Components|TextRender|SetText (Variables|Default|GetTextReff) (|GenerictoText (Utilities|String|Append (Utilities|String|ToString(Text) (Utilities|Text|ToText(Float) (/ (Variables|Default|GetSegmentLengthUU) 1e+02) "HalfToEven" false true 1 324 2 2)) "m")))))))))